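; BP_Iteam is an inventory item actor that takes its appearance and type from a Data Table row.
; The construction script calls SetMesh, which looks up the row through the Item struct's ItemID handle, applies its mesh and copies its ItemTypes into Item.
; GetIteam exposes that struct, while the health and money getters are stubs and the event graph has no logic.
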(event `self.ReceiveTick`
  (params (DeltaSeconds :type "Float (single-precision)")))

(fn `Get Select DT`
  (returns (OutDataTable :type "/Game/Inventory/Structs/S_Item Structure"))
  (bind _item_itemid (break `/Game/Inventory/Structs/S_Slot` (`self.Item`)))
  (bind (_datatable _rowname) (break `DataTableRowHandle` _item_itemid))
  (bind _returnvalue (`|GetDataTableRow` _datatable _rowname)
    (:`then`
      (return _returnvalue))))

(fn `GetHealth`
  (returns (Value :type "Float (double-precision)"))
  (return 0.0))

(fn `GetIteam`
  (returns (Data :type "/Game/Inventory/Structs/S_Slot Structure"))
  (return (`self.Item`)))

(fn `GetMaxHealth`
  (returns (Value :type "Float (double-precision)"))
  (return 0.0))

(fn `GetMoneyDT`
  (returns (OutDataTable :type "/Game/Inventory/Structs/S_Money Structure"))
  (return))

(fn `SetMesh`
  (bind ((`Mesh_16_28A1A8BD490142162D3132B706D4E2AA` _mesh) (`ItemTypes_19_036D67DA4A36D959ED5E868A8DC79DF7` _itemtypes)) (break `/Game/Inventory/Structs/S_Item` (`self.Get Select DT`)))
  (`StaticMeshComponent.SetStaticMesh` (`self.StaticMesh`) _mesh)
  (setmembers `/Game/Inventory/Structs/S_Slot` :`StructRef` (`self.Item`) :`ItemTypes` _itemtypes))

(fn `UserConstructionScript`
  (`self.SetMesh`))
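; BP_Money is an inventory money actor whose appearance is driven by a data table.
; On construction, SetMoneyMesh calls GetSelectDT to look up the row named by the Money row handle and applies that row's Mesh to the SMMoney static mesh component.
; GetModuleName returns the module path Inventory.Blueprints.BP_Money, and the event graph holds no gameplay logic.
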(event `self.ReceiveBeginPlay`)

(fn `GetModuleName`
  (returns (ReturnValue :type String))
  (return "Inventory.Blueprints.BP_Money"))

(fn `GetSelectDT`
  (returns (OutDataTable :type "/Game/Inventory/Structs/S_Money Structure"))
  (bind (_money_datatable _money_rowname) (break `DataTableRowHandle` (`self.Money`)))
  (bind _returnvalue (`|GetDataTableRow` _money_datatable _money_rowname)
    (:`then`
      (return _returnvalue))))

(fn `SetMoneyMesh`
  (bind (_outdatatable_name _outdatatable_amount _outdatatable_mesh) (break `/Game/Inventory/Structs/S_Money` (`self.GetSelectDT`)))
  (`StaticMeshComponent.SetStaticMesh` (`self.SM_Money`) _outdatatable_mesh))

(fn `UserConstructionScript`
  (`self.SetMoneyMesh`))
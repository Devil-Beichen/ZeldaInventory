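; Player inventory component that manages money pickup, health and their UI widgets.
; On BeginPlay it adds the inventory input mapping, creates the inventory and health bar widgets, and binds owner overlap.
; Overlaps use interface messages to read and destroy money actors, passing the running total to the inventory widget.
; IA_Inventory opens that widget in UI-only mode, while N and M adjust clamped health and refresh the bar.
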(event `self.ReceiveBeginPlay`
  (bind _returnvalue (`GameplayStatics.GetPlayerControllerFromID` 0))
  (add `Actor.OnActorBeginOverlap` (`self.GetOwner`) (`|CreateDelegate` :!event `OnBeginOverlap`))
  (`EnhancedInputSubsystemInterface.AddMappingContext` (pcsubsystem `EnhancedInputLocalPlayerSubsystem` _returnvalue) "/Game/Inventory/Inputs/IMC_Inventory.IMC_Inventory" 0 (struct))
  (bind _returnvalue_2 (`|CreateWidget` "/Game/Inventory/Widgets/WBP_Inventory.WBP_Inventory_C" _returnvalue))
  (set `self.WBP_Inventory` _returnvalue_2)
  (`self.HelathBarInit`))

(event `/Game/Inventory/Interfaces/BI_Zelda.IncreaseHelath`
  (params (HelathToIncrease :type "Float (double-precision)"))
  (set `self.Health` (`KismetMathLibrary.FClamp` (+ HelathToIncrease (`self.Health`)) 0.0 (`self.MaxHealth`))))

(event `/Game/Inventory/Interfaces/BI_Zelda.DecreaseHelath`
  (params (HelathToDecrease :type "Float (double-precision)"))
  (set `self.Health` (`KismetMathLibrary.FClamp` (- (`self.Health`) HelathToDecrease) 0.0 (`self.MaxHealth`))))

(event `Key|N`
  (params (Key :type "Key Structure"))
  (:`Pressed`
    (message `/Game/Inventory/Interfaces/BI_Zelda.IncreaseHelath` self 0.5)
    (bind _wbp_healthbar (`self.WBP_HealthBar` :!label _label)
      (:`then`
        (`/Game/Inventory/Widgets/WBP_HealthBar.UpdateHealthBar` _wbp_healthbar))
      (:`else`))))

(event `Key|M`
  (params (Key :type "Key Structure"))
  (:`Pressed`
    (message `/Game/Inventory/Interfaces/BI_Zelda.DecreaseHelath` self 0.5)
    (goto _label)))

(event `EnhancedInput|/Game/Inventory/Inputs/IA_Inventory`
  (params (ActionValue :type Boolean) (ElapsedSeconds :type "Float (double-precision)") (TriggeredSeconds :type "Float (double-precision)") (InputAction :type "InputAction Object Reference" :default "/Game/Inventory/Inputs/IA_Inventory.IA_Inventory"))
  (bind _returnvalue (`GameplayStatics.GetPlayerControllerFromID` 0))
  (:`Triggered`
    (bind _wbp_inventory (`self.WBP_Inventory`)
      (:`then`
        (`UserWidget.AddToViewport` _wbp_inventory 0)
        (set `PlayerController.bShowMouseCursor` true _returnvalue)
        (`WidgetBlueprintLibrary.SetInputMode_UIOnlyEx` _returnvalue _wbp_inventory))
      (:`else`))))

(fn `GetHealth`
  (returns (Value :type "Float (double-precision)"))
  (return (`self.Health`)))

(fn `GetMaxHealth`
  (returns (Value :type "Float (double-precision)"))
  (return (`self.MaxHealth`)))

(fn `GetMoneyDT`
  (returns (OutDataTable :type "/Game/Inventory/Structs/S_Money Structure"))
  (return))

(fn `HelathBarInit`
  (bind _returnvalue (`|CreateWidget` "/Game/Inventory/Widgets/WBP_HealthBar.WBP_HealthBar_C" (`GameplayStatics.GetPlayerControllerFromID` 0)))
  (bind _output_get (set `self.WBP_HealthBar` _returnvalue))
  (`UserWidget.SetPositionInViewport` _output_get (10.0 10.0) true)
  (`UserWidget.AddToViewport` _output_get 0))

(fn `OnBeginOverlap`
  (params (OverlappedActor :type "Actor Object Reference") (OtherActor :type "Actor Object Reference"))
  (`self.PickUpMoney` OtherActor))

(fn `PickUpMoney`
  (params (Actor :type "Actor Object Reference"))
  (bind _outdatatable (message `/Game/Inventory/Interfaces/BI_Zelda.GetMoneyDT` Actor))
  (set `self.MoneyAmount` (+ (`.Amount_6_73C44FCF41562574E57F9CA5D569ABA5` (break `/Game/Inventory/Structs/S_Money` _outdatatable)) (`self.MoneyAmount`)))
  (`|ExecutionSequence`
    (:`then_0`
      (bind _wbp_inventory (`self.WBP_Inventory`)
        (:`then`
          (set `/Game/Inventory/Widgets/WBP_Inventory.MoneyAmount` (`self.MoneyAmount`) _wbp_inventory))
        (:`else`)))
    (:`then_1`
      (message `/Game/Inventory/Interfaces/BI_Zelda.DestroyMoney` Actor))))